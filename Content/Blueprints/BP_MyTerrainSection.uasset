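; A terrain section actor that makes sure its generated meshes have a landscape material at runtime.
; After a short delay on BeginPlay, it checks the base and four LOD components in both the RuntimeMesh and ProceduralMesh sets.
; Any component without a valid material in slot 0 receives MI_Landscape_100, while existing materials are left untouched.
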(event EventBeginPlay
  (Utilities|FlowControl|Delay 0.2)
  (for _array_element (Utilities|Array|MakeArray (Variables|Default|GetRuntimeMeshComponent) (Variables|Default|GetRuntimeMeshComponentLOD1) (Variables|Default|GetRuntimeMeshComponentLOD2) (Variables|Default|GetRuntimeMeshComponentLOD3) (Variables|Default|GetRuntimeMeshComponentLOD4))
    (Utilities|IsValid (Rendering|Material|GetMaterial _array_element 0)
      (:Is%20Not%20Valid
        (Rendering|Material|SetMaterial _array_element 0 "/Game/Materials/MI_Landscape_100.MI_Landscape_100"))))
  (for _array_element_2 (Utilities|Array|MakeArray (Variables|Default|GetProceduralMeshComponent) (Variables|Default|GetProceduralMeshComponentLOD1) (Variables|Default|GetProceduralMeshComponentLOD2) (Variables|Default|GetProceduralMeshComponentLOD3) (Variables|Default|GetProceduralMeshComponentLOD4))
    (Utilities|IsValid (Rendering|Material|GetMaterial _array_element_2 0)
      (:Is%20Not%20Valid
        (Rendering|Material|SetMaterial _array_element_2 0 "/Game/Materials/MI_Landscape_100.MI_Landscape_100")))))

(fn ConstructionScript)