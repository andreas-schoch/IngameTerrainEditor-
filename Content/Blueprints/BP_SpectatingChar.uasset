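; Free-flying spectator character for terrain sculpting, with mouse-wheel speed control and a HUD bound to its Sculpt component.
; Each tick it feeds the cursor hit to Sculpt and moves a decal brush there, scaled and shaded by radius and falloff.
; Holding Fire sculpts and locks camera look, with a short debounced release.
; Debug keys spawn erosion test actors at camera trace hits or draw a terrain normal estimated from neighbouring height traces.
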(event EventBeginPlay
  (bind _returnvalue (Game|GetPlayerController 0))
  (bind _returnvalue_2 (UserInterface|CreateWidget "/Game/Blueprints/WBP_HUD.WBP_HUD_C" 0 (Variables|Default|GetSculpt) 5e+03 1e+03))
  (UserInterface|Viewport|AddtoViewport _returnvalue_2 0)
  (Variables|Default|SetHUDRef _returnvalue_2)
  (Input|SetInputModeGameandUI _returnvalue _returnvalue_2 "DoNotLock" false)
  (Variables|/Script/Engine.PlayerController|SetbShowMouseCursor _returnvalue true)
  (bind _returnvalue_3 (Game|SpawnActorfromClass "/Game/Blueprints/BP_TerrainDecalActor.BP_TerrainDecalActor_C" (Math|Transform|MakeTransform "0, 0, 0") "AlwaysSpawn" 0 0))
  (Variables|Default|SetDecalBrush _returnvalue_3)
  (bind _returnvalue_4 (AddComponent|AddChildActorComponent _returnvalue_3 true))
  (Variables|Default|SetChildActorDecal _returnvalue_4)
  (bind _returnvalue_5 (Rendering|Material|CreateDynamicMaterialInstance "/Game/Materials/MI_DecalBrush.MI_DecalBrush" :!class /Script/Engine.KismetMaterialLibrary))
  (Variables|Default|SetDecalMatInstance _returnvalue_5)
  (Rendering|Components|Decal|SetDecalMaterial (Variables|/Script/Engine.DecalActor|GetDecal (Variables|Default|GetDecalBrush)) (Variables|Default|GetDecalMatInstance)))

(event EventTick
  (params (DeltaSeconds :type Float%20%28single-precision%29))
  (bind _returnvalue (Game|GetPlayerController 0))
  (bind _sculpt (Variables|Default|GetSculpt))
  (bind _hitresult (Game|Player|GetHitResultUnderCursorbyChannel _returnvalue "TraceTypeQuery1" true))
  (bind _sculptsettings (Variables|/Script/RuntimeMeshTerrain.SculptComponent|GetSculptSettings _sculpt))
  (bind _returnvalue_2 (/ (.sculptradius _sculptsettings) 5e+01))
  (Utilities|FlowControl|Sequence
    (:then_0
      (Utilities|IsValid (Variables|Default|GetDecalBrush)
        (:Is%20Valid
          (Transformation|SetActorLocation (Variables|Default|GetDecalBrush) (.Location (Collision|BreakHitResult _hitresult)) false false)
          (Transformation|SetActorScale3D (Variables|Default|GetDecalBrush) (Math|Vector|MakeVector 5e+02 _returnvalue_2 _returnvalue_2))
          (Rendering|Material|SetScalarParameterValue (Variables|Default|GetDecalMatInstance) "InnerCircle" (- (/ (.falloff _sculptsettings) 2.0) 0.01) :!class /Script/Engine.MaterialInstanceDynamic))
        (:Is%20Not%20Valid
          (bind _outactors (Actor|GetAllActorsOfClass "/Game/Blueprints/BP_TerrainDecalActor.BP_TerrainDecalActor_C"))
          (Variables|Default|SetDecalBrush (Utilities|Array|Get(acopy) _outactors))
          (bind _returnvalue_3 (Rendering|Material|CreateDynamicMaterialInstance "/Game/Materials/MI_DecalBrush.MI_DecalBrush" :!class /Script/Engine.KismetMaterialLibrary))
          (Variables|Default|SetDecalMatInstance _returnvalue_3)
          (Rendering|Components|Decal|SetDecalMaterial (Variables|/Script/Engine.DecalActor|GetDecal (Variables|Default|GetDecalBrush)) (Variables|Default|GetDecalMatInstance)))))
    (:then_1
      (Class|SculptComponent|SetHitResult (Variables|Default|GetSculpt) _hitresult))))

(event Input|ActionEvents|InputActionFire
  (params (Key :type Key%20Structure :default "AnyKey"))
  ;[1 1 1] LMB
  (:Pressed
    (Variables|Default|SetLMBDown true)
    (Variables|Default|SetDisableCameraMovement true)
    ;[1 1 1] Sculpt
    (Class|SculptComponent|SculptStart (Variables|Default|GetSculpt)))
  (:Released
    (bind _output_get (Variables|Default|SetLMBDown false))
    (Utilities|FlowControl|Delay 0.05)
    (if (not _output_get)
      (Variables|Default|SetDisableCameraMovement false)
      (Class|SculptComponent|SculptStop (Variables|Default|GetSculpt)))))

(event Input|AxisEvents|InputAxisTurn
  (params (AxisValue :type Float%20%28single-precision%29))
  ;[1 1 1] Camera
  (if (not (Variables|Default|GetDisableCameraMovement))
    (Pawn|Input|AddControllerYawInput AxisValue)))

(event Input|AxisEvents|InputAxisMoveUp
  (params (AxisValue :type Float%20%28single-precision%29))
  ;[1 1 1] Movement
  (Pawn|Input|AddMovementInput (Math|Vector|GetUpVector (Math|Rotator|MakeRotator 0.0 0.0 (.yaw (Pawn|GetControlRotation :!class /Script/Engine.Pawn)))) AxisValue false))

(event Input|AxisEvents|InputAxisLookUp
  (params (AxisValue :type Float%20%28single-precision%29))
  ;[1 1 1] Camera
  (if (not (Variables|Default|GetDisableCameraMovement))
    (Pawn|Input|AddControllerPitchInput AxisValue)))

(event Input|AxisEvents|InputAxisMoveForward
  (params (AxisValue :type Float%20%28single-precision%29))
  ;[1 1 1] Movement
  (Pawn|Input|AddMovementInput (Math|Vector|GetForwardVector (Pawn|GetControlRotation :!class /Script/Engine.Pawn)) AxisValue false))

(event Input|AxisEvents|InputAxisMoveRight
  (params (AxisValue :type Float%20%28single-precision%29))
  ;[1 1 1] Movement
  (Pawn|Input|AddMovementInput (Math|Vector|GetRightVector (Pawn|GetControlRotation :!class /Script/Engine.Pawn)) AxisValue false))

(event Input|KeyboardEvents|Z
  (params (Key :type Key%20Structure :default "AnyKey"))
  (bind _camera (Variables|Default|GetCamera))
  (bind _returnvalue (Transformation|GetWorldLocation _camera))
  (:Pressed
    (bind _outhit (Collision|LineTraceByChannel _returnvalue (+ _returnvalue (* (Math|Vector|GetForwardVector _camera) 1e+05)) "TraceTypeQuery2" true 0 "ForDuration" false))
    (Game|SpawnActorfromClass "/Game/Blueprints/BP_ErosionTest2.BP_ErosionTest2_C" (Math|Transform|MakeTransform (+ (.location _outhit) "0, 0,300.000000") "0, 0, 0" "1,1,1") "Undefined" 0 0)))

(event Input|KeyboardEvents|U
  (params (Key :type Key%20Structure :default "AnyKey"))
  (bind _camera (Variables|Default|GetCamera))
  (bind _returnvalue (Transformation|GetWorldLocation _camera))
  (:Pressed
    (bind _outhit (Collision|LineTraceByChannel _returnvalue (+ _returnvalue (* (Math|Vector|GetForwardVector _camera) 1e+05)) "TraceTypeQuery2" true 0 "ForDuration" false))
    (Game|SpawnActorfromClass "/Game/Blueprints/BP_ErosionTest1.BP_ErosionTest1_C" (Math|Transform|MakeTransform (+ (.location _outhit) "0, 0,100.000000") "0, 0, 0" "1,1,1") "Undefined" 0 0)))

(event Input|KeyboardEvents|I
  (params (Key :type Key%20Structure :default "AnyKey"))
  (bind _camera (Variables|Default|GetCamera))
  (bind _grid (Variables|Default|GetGrid))
  (bind _returnvalue (Transformation|GetWorldLocation _camera))
  ;[1 1 1] Get Normal test
  (:Pressed
    (bind _outhit (Collision|LineTraceByChannel _returnvalue (+ _returnvalue (* (Math|Vector|GetForwardVector _camera) 1e+05)) "TraceTypeQuery1" false 0 "ForDuration"))
    (Variables|Default|SetHitNormal (.normal _outhit))
    (Variables|Default|SetCenter (Math|Vector|MakeVector (Math|Float|SnapToGrid(Float) (.X (Math|Vector|BreakVector (.location _outhit))) _grid) (Math|Float|SnapToGrid(Float) (.Y (Math|Vector|BreakVector (.location _outhit))) _grid) (+ (.Z (Math|Vector|BreakVector (.location _outhit))) 5e+02)))
    (for (_array_element _array_index) (Utilities|Array|MakeArray "1.000000,0.000000, 0" "-1.000000,1.000000, 0" "0.000000,1.000000, 0" "0,-1.000000, 0")
      (bind _outhit_2 (Collision|LineTraceByChannel (+ (* _array_element (Variables|Default|GetGrid)) (Variables|Default|GetCenter)) (+ (+ (* _array_element (Variables|Default|GetGrid)) (Variables|Default|GetCenter)) "0, 0,-1000.000000") "TraceTypeQuery1" false 0 "ForOneFrame"))
      (switch int _array_index
        (:0
          (Variables|Default|SetHeightUP (.Z (Math|Vector|BreakVector (.location _outhit_2)))))
        (:1
          (Variables|Default|SetHeightDown (.Z (Math|Vector|BreakVector (.location _outhit_2)))))
        (:2
          (Variables|Default|SetHeightRight (.Z (Math|Vector|BreakVector (.location _outhit_2)))))
        (:3
          (Variables|Default|SetHeightLeft (.Z (Math|Vector|BreakVector (.location _outhit_2)))))))
    (Variables|Default|SetNewVar_0 (Math|Vector|Normalize (Math|Vector|MakeVector (- (Variables|Default|GetHeightDown) (Variables|Default|GetHeightUP)) (- (Variables|Default|GetHeightLeft) (Variables|Default|GetHeightRight)) 0.0)))
    (bind _output_get (Variables|Default|SetNormal (Math|Vector|Normalize (Math|Vector|MakeVector (- (Variables|Default|GetHeightUP) (Variables|Default|GetHeightDown)) (- (Variables|Default|GetHeightRight) (Variables|Default|GetHeightLeft)) 2.0))))
    (Development|PrintString (Utilities|String|ToString(Vector) _output_get) true true "(R=1.000000,G=0.000000,B=0.153831,A=1.000000)")
    (Development|PrintString (Utilities|String|ToString(Vector) (Variables|Default|GetNewVar_0)) true true "(R=0.000000,G=0.319231,B=1.000000,A=1.000000)")
    (Rendering|Debug|DrawDebugLine (- (Variables|Default|GetCenter) "0, 0,500.000000") (+ (- (Variables|Default|GetCenter) "0, 0,500.000000") (* (Variables|Default|GetNormal) 5e+02)) "(R=0.000000,G=1.000000,B=0.040460,A=1.000000)" 15.0 9.0)
    (Rendering|Debug|DrawDebugLine (- (Variables|Default|GetCenter) "0, 0,500.000000") (+ (- (Variables|Default|GetCenter) "0, 0,500.000000") (* (Variables|Default|GetHitNormal) 2.5e+02)) "(R=1.000000,G=0.000000,B=0.172772,A=1.000000)" 15.0 9.0)
    (Rendering|Debug|DrawDebugLine (- (Variables|Default|GetCenter) "0, 0,500.000000") (+ (- (Variables|Default|GetCenter) "0, 0,500.000000") (* (Variables|Default|GetNewVar_0) 4e+02)) "(R=0.000000,G=0.185775,B=1.000000,A=1.000000)" 15.0 9.0)))

(event Input|MouseEvents|MouseWheelDown
  (params (Key :type Key%20Structure :default "AnyKey"))
  (bind _charactermovement (Variables|Character|GetCharacterMovement))
  (:Pressed
    (Variables|/Script/Engine.CharacterMovementComponent|SetMaxFlySpeed _charactermovement (Math|Float|Clamp(Float) (- (Variables|/Script/Engine.CharacterMovementComponent|GetMaxFlySpeed _charactermovement) 1e+03) 1e+03 1e+05))
    (Variables|/Script/Engine.CharacterMovementComponent|SetMaxAcceleration _charactermovement (Math|Float|Clamp(Float) (- (Variables|/Script/Engine.CharacterMovementComponent|GetMaxFlySpeed _charactermovement) 1e+03) 1e+03 1e+05))))

(event Input|MouseEvents|MouseWheelUp
  (params (Key :type Key%20Structure :default "AnyKey"))
  (bind _charactermovement (Variables|Character|GetCharacterMovement))
  (:Pressed
    (Variables|/Script/Engine.CharacterMovementComponent|SetMaxFlySpeed _charactermovement (Math|Float|Clamp(Float) (+ (Variables|/Script/Engine.CharacterMovementComponent|GetMaxFlySpeed _charactermovement) 1e+03) 1e+03 1e+05))
    (Variables|/Script/Engine.CharacterMovementComponent|SetMaxAcceleration _charactermovement (Math|Float|Clamp(Float) (+ (Variables|/Script/Engine.CharacterMovementComponent|GetMaxFlySpeed _charactermovement) 1e+03) 1e+03 1e+05))))

(fn ConstructionScript)