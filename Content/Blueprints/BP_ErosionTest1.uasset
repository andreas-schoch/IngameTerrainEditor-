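; Erosion test actor that walks downhill over terrain like a droplet, starting its Sculpt component after a short delay and expiring ten seconds later.
; Each Tick it line-traces eight nearby grid directions, picks the lowest hit and steps GridSize that way, hovering just above that height.
; It resets the camera's rotation after each step and draws debug lines for the hit normal and camera forward vector.
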(event EventBeginPlay
  (Utilities|FlowControl|Delay 1.0)
  (Variables|Default|Setstart true)
  (Actor|SetLifeSpan 1e+01)
  (Class|SculptComponent|SculptStart (Variables|Default|GetSculpt)))

(event EventTick
  (params (DeltaSeconds :type Float%20%28single-precision%29))
  (bind _returnvalue (Transformation|GetActorLocation))
  (bind _camera (Variables|Default|GetCamera))
  (bind _returnvalue_2 (Transformation|GetWorldLocation _camera))
  (Utilities|FlowControl|Sequence
    (:then_0
      (if (Variables|Default|Getstart)
        (Variables|Default|SetTemp (+ (* (Transformation|GetWorldLocation (Variables|Default|GetStaticMesh)) "0, 0,1.000000") 3e+03))
        (Variables|Default|SetIndex -1)
        (for _index (range 0 7)
          (bind _outhit (Collision|LineTraceByChannel (+ (+ (* (Utilities|Select :Index _index :Option%200 "1.000000,-1.000000,0" :Option%201 "1.000000,0,0" :Option%202 "1.000000,1.000000,0" :Option%203 "0.000000,-1.000000,0" :Option%204 "0,1.000000,0" :Option%205 "-1.000000,-1.000000,0" :Option%206 "-1.000000,0,0" :Option%207 "-1.000000,1.000000,0") 5) (Transformation|GetWorldLocation (Variables|Default|GetStaticMesh))) "0, 0,500.000000") (- (+ (* (Utilities|Select :Index _index :Option%200 "1.000000,-1.000000,0" :Option%201 "1.000000,0,0" :Option%202 "1.000000,1.000000,0" :Option%203 "0.000000,-1.000000,0" :Option%204 "0,1.000000,0" :Option%205 "-1.000000,-1.000000,0" :Option%206 "-1.000000,0,0" :Option%207 "-1.000000,1.000000,0") 5) (Transformation|GetWorldLocation (Variables|Default|GetStaticMesh))) "0, 0,500.000000") "TraceTypeQuery1" true 0 "None"))
          (if (and (.bBlockingHit (Collision|BreakHitResult _outhit)) (< (.z (.Location (Collision|BreakHitResult _outhit))) (.z (Variables|Default|GetTemp))))
            (Variables|Default|SetTemp (Math|Vector|MakeVector 0.0 0.0 (.z (.Location (Collision|BreakHitResult _outhit)))))
            (Variables|Default|SetIndex _index)
            (Variables|Default|SetTempNormal (.Normal (Collision|BreakHitResult _outhit)))))
        (if (!= (Variables|Default|GetIndex) -1)
          (Transformation|SetActorLocation (+ (* (Utilities|Select :Index (Variables|Default|GetIndex) :Option%200 "1.000000,-1.000000,0" :Option%201 "1.000000,0,0" :Option%202 "1.000000,1.000000,0" :Option%203 "0.000000,-1.000000,0" :Option%204 "0,1.000000,0" :Option%205 "-1.000000,-1.000000,0" :Option%206 "-1.000000,0,0" :Option%207 "-1.000000,1.000000,0") (Variables|Default|GetGridSize)) (Math|Vector|MakeVector (.x _returnvalue) (.y _returnvalue) (+ (.z (Variables|Default|GetTemp)) 5e+01))) false false)
          (Rendering|Debug|DrawDebugLine (+ (* (Utilities|Select :Index (Variables|Default|GetIndex) :Option%200 "1.000000,-1.000000,0" :Option%201 "1.000000,0,0" :Option%202 "1.000000,1.000000,0" :Option%203 "0.000000,-1.000000,0" :Option%204 "0,1.000000,0" :Option%205 "-1.000000,-1.000000,0" :Option%206 "-1.000000,0,0" :Option%207 "-1.000000,1.000000,0") (Variables|Default|GetGridSize)) (Math|Vector|MakeVector (.x _returnvalue) (.y _returnvalue) (+ (.z (Variables|Default|GetTemp)) 5e+01))) (+ (+ (* (Utilities|Select :Index (Variables|Default|GetIndex) :Option%200 "1.000000,-1.000000,0" :Option%201 "1.000000,0,0" :Option%202 "1.000000,1.000000,0" :Option%203 "0.000000,-1.000000,0" :Option%204 "0,1.000000,0" :Option%205 "-1.000000,-1.000000,0" :Option%206 "-1.000000,0,0" :Option%207 "-1.000000,1.000000,0") (Variables|Default|GetGridSize)) (Math|Vector|MakeVector (.x _returnvalue) (.y _returnvalue) (+ (.z (Variables|Default|GetTemp)) 5e+01))) (* (Variables|Default|GetTempNormal) 3e+02)) "(R=0.049005,G=0.204401,B=0.535000,A=1.000000)" 1.0 15.0)
          (Transformation|SetWorldRotation (Variables|Default|GetCamera) "-90.000000, 0, 0" false false))))
    (:then_1
      (Rendering|Debug|DrawDebugLine :LineStart _returnvalue_2 :LineEnd (+ _returnvalue_2 (* (Math|Vector|GetForwardVector _camera) 5e+03)) :Duration 1.0 :Thickness 35.0))))

(fn ConstructionScript)