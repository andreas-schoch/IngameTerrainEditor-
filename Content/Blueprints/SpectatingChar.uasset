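; Player-controlled spectator character for terrain sculpting, with free movement and a HUD bound to its Sculpt component.
; Holding Fire runs sculpting from the camera and locks look input until shortly after release.
; A spawned decal actor follows the sculpt location each tick, with scale and inner circle driven by radius and falloff.
; Debug keys U and I trace grid-snapped neighbour points to compare terrain normals from cross products and height differences.
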(event EventBeginPlay
  (bind _returnvalue (Game|GetPlayerController 0))
  (bind _returnvalue_2 (UserInterface|CreateWidget "/Game/Blueprints/HUD.HUD_C" 0 (Variables|Default|GetSculpt)))
  (UserInterface|Viewport|AddtoViewport _returnvalue_2 0)
  (Variables|Default|SetHUDRef _returnvalue_2)
  (Input|SetInputModeGameandUI _returnvalue _returnvalue_2 "DoNotLock" false)
  (Variables|/Script/Engine.PlayerController|SetbShowMouseCursor _returnvalue true)
  (bind _returnvalue_3 (Game|SpawnActorfromClass "/Game/Blueprints/TerrainDecalActor.TerrainDecalActor_C" (Math|Transform|MakeTransform "0, 0, 0") "AlwaysSpawn" 0 0))
  (Variables|Default|SetDecalBrush _returnvalue_3)
  (bind _returnvalue_4 (AddComponent|AddChildActorComponent _returnvalue_3 true))
  (Variables|Default|SetChildActorDecal _returnvalue_4)
  (bind _returnvalue_5 (Rendering|Material|CreateDynamicMaterialInstance "/Game/Materials/DecalTest_Inst.DecalTest_Inst" :!class /Script/Engine.KismetMaterialLibrary))
  (Variables|Default|SetDecalMatInstance _returnvalue_5)
  (Rendering|Components|Decal|SetDecalMaterial (Variables|/Script/Engine.DecalActor|GetDecal (Variables|Default|GetDecalBrush)) (Variables|Default|GetDecalMatInstance)))

(event EventTick
  (params (DeltaSeconds :type Float%20%28single-precision%29))
  (bind _sculpt (Variables|Default|GetSculpt))
  (bind _sculptsettings (Variables|/Script/RuntimeMeshTerrain.SculptComponent|GetSculptSettings _sculpt))
  (bind _returnvalue (/ (.sculptradius _sculptsettings) 1e+02))
  (bind _returnvalue_2 (* _returnvalue 2.0))
  (Utilities|FlowControl|Sequence
    (:then_0
      (Utilities|IsValid (Variables|Default|GetDecalBrush)
        (:Is%20Valid
          (Transformation|SetActorLocation (Variables|Default|GetDecalBrush) (Variables|/Script/RuntimeMeshTerrain.SculptComponent|GetCurrentSculptLocation _sculpt) false false)
          (Transformation|SetActorScale3D (Variables|Default|GetDecalBrush) (Math|Vector|MakeVector 5e+02 _returnvalue_2 _returnvalue_2))
          (Rendering|Material|SetScalarParameterValue (Variables|Default|GetDecalMatInstance) "InnerCircle" (- (/ (.falloff (Variables|/Script/RuntimeMeshTerrain.SculptComponent|GetSculptSettings (Variables|Default|GetSculpt))) 2.0) 0.01) :!class /Script/Engine.MaterialInstanceDynamic))
        (:Is%20Not%20Valid
          (bind _outactors (Actor|GetAllActorsOfClass "/Game/Blueprints/TerrainDecalActor.TerrainDecalActor_C"))
          (Variables|Default|SetDecalBrush (Utilities|Array|Get(acopy) _outactors))
          (bind _returnvalue_3 (Rendering|Material|CreateDynamicMaterialInstance "/Game/Materials/DecalTest_Inst.DecalTest_Inst" :!class /Script/Engine.KismetMaterialLibrary))
          (Variables|Default|SetDecalMatInstance _returnvalue_3)
          (Rendering|Components|Decal|SetDecalMaterial (Variables|/Script/Engine.DecalActor|GetDecal (Variables|Default|GetDecalBrush)) (Variables|Default|GetDecalMatInstance)))))))

(event Input|ActionEvents|InputActionFire
  (params (Key :type Key%20Structure :default "AnyKey"))
  ;[1 1 1] LMB
  (:Pressed
    (Variables|Default|SetLMBDown true)
    (Variables|Default|SetDisableCameraMovement true)
    ;[1 1 1] Sculpt
    (Class|SculptComponent|SculptStart (Variables|Default|GetSculpt) (Variables|Default|GetCamera)))
  (:Released
    (bind _output_get (Variables|Default|SetLMBDown false))
    (Utilities|FlowControl|Delay 0.05)
    (if (not _output_get)
      (Variables|Default|SetDisableCameraMovement false)
      (Class|SculptComponent|SculptStop (Variables|Default|GetSculpt)))))

(event Input|AxisEvents|InputAxisTurn
  (params (AxisValue :type Float%20%28single-precision%29))
  ;[1 1 1] Camera
  (if (not (Variables|Default|GetDisableCameraMovement))
    (Pawn|Input|AddControllerYawInput AxisValue)))

(event Input|AxisEvents|InputAxisMoveUp
  (params (AxisValue :type Float%20%28single-precision%29))
  ;[1 1 1] Movement
  (Pawn|Input|AddMovementInput (Math|Vector|GetUpVector (Math|Rotator|MakeRotator 0.0 0.0 (.yaw (Pawn|GetControlRotation :!class /Script/Engine.Pawn)))) AxisValue false))

(event Input|AxisEvents|InputAxisLookUp
  (params (AxisValue :type Float%20%28single-precision%29))
  ;[1 1 1] Camera
  (if (not (Variables|Default|GetDisableCameraMovement))
    (Pawn|Input|AddControllerPitchInput AxisValue)))

(event Input|AxisEvents|InputAxisMoveForward
  (params (AxisValue :type Float%20%28single-precision%29))
  ;[1 1 1] Movement
  (Pawn|Input|AddMovementInput (Math|Vector|GetForwardVector (Pawn|GetControlRotation :!class /Script/Engine.Pawn)) AxisValue false))

(event Input|AxisEvents|InputAxisMoveRight
  (params (AxisValue :type Float%20%28single-precision%29))
  ;[1 1 1] Movement
  (Pawn|Input|AddMovementInput (Math|Vector|GetRightVector (Pawn|GetControlRotation :!class /Script/Engine.Pawn)) AxisValue false))

(event Input|MouseEvents|RightMouseButton
  (params (Key :type Key%20Structure :default "AnyKey")))

(event Input|KeyboardEvents|U
  (params (Key :type Key%20Structure :default "AnyKey"))
  (bind _grid (Variables|Default|GetGrid))
  (bind _camera (Variables|Default|GetCamera))
  (bind _returnvalue (Transformation|GetWorldLocation _camera))
  (:Pressed
    (bind _outhit (Collision|LineTraceByChannel _returnvalue (+ _returnvalue (* (Math|Vector|GetForwardVector _camera) 1e+05)) "TraceTypeQuery1" false 0 "ForDuration"))
    (Variables|Default|SetHitNormal (.normal _outhit))
    (Variables|Default|SetCenter (Math|Vector|MakeVector (Math|Float|SnapToGrid(Float) (.X (Math|Vector|BreakVector (.location _outhit))) _grid) (Math|Float|SnapToGrid(Float) (.Y (Math|Vector|BreakVector (.location _outhit))) _grid) (+ (.Z (Math|Vector|BreakVector (.location _outhit))) 5e+02)))
    (for (_array_element _array_index) (Utilities|Array|MakeArray "1.000000,0.000000, 0" "-1.000000,1.000000, 0" "0.000000,1.000000, 0" "0,-1.000000, 0")
      (bind _outhit_2 (Collision|LineTraceByChannel (+ (* _array_element (Variables|Default|GetGrid)) (Variables|Default|GetCenter)) (+ (+ (* _array_element (Variables|Default|GetGrid)) (Variables|Default|GetCenter)) "0, 0,-1000.000000") "TraceTypeQuery1" false 0 "ForOneFrame"))
      (switch int _array_index
        (:0
          (Variables|Default|SetU (.location _outhit_2)))
        (:1
          (Variables|Default|SetD (.location _outhit_2)))
        (:2
          (Variables|Default|SetR (.location _outhit_2)))
        (:3
          (Variables|Default|SetL (.location _outhit_2)))))
    (Variables|Default|SetNormal (Math|Vector|Normalize (Math|Vector|CrossProduct (- (Variables|Default|GetU) (Variables|Default|GetD)) (- (Variables|Default|GetR) (Variables|Default|GetL)))))
    (Rendering|Debug|DrawDebugLine (- (Variables|Default|GetCenter) "0, 0,500.000000") (+ (- (Variables|Default|GetCenter) "0, 0,500.000000") (* (Variables|Default|GetNormal) 5e+02)) "(R=0.908660,G=1.000000,B=0.000000,A=1.000000)" 15.0 9.0)))

(event Input|KeyboardEvents|I
  (params (Key :type Key%20Structure :default "AnyKey"))
  (bind _camera (Variables|Default|GetCamera))
  (bind _grid (Variables|Default|GetGrid))
  (bind _returnvalue (Transformation|GetWorldLocation _camera))
  (:Pressed
    (bind _outhit (Collision|LineTraceByChannel _returnvalue (+ _returnvalue (* (Math|Vector|GetForwardVector _camera) 1e+05)) "TraceTypeQuery1" false 0 "ForDuration"))
    (Variables|Default|SetHitNormal (.normal _outhit))
    (Variables|Default|SetCenter (Math|Vector|MakeVector (Math|Float|SnapToGrid(Float) (.X (Math|Vector|BreakVector (.location _outhit))) _grid) (Math|Float|SnapToGrid(Float) (.Y (Math|Vector|BreakVector (.location _outhit))) _grid) (+ (.Z (Math|Vector|BreakVector (.location _outhit))) 5e+02)))
    (for (_array_element _array_index) (Utilities|Array|MakeArray "1.000000,0.000000, 0" "-1.000000,1.000000, 0" "0.000000,1.000000, 0" "0,-1.000000, 0")
      (bind _outhit_2 (Collision|LineTraceByChannel (+ (* _array_element (Variables|Default|GetGrid)) (Variables|Default|GetCenter)) (+ (+ (* _array_element (Variables|Default|GetGrid)) (Variables|Default|GetCenter)) "0, 0,-1000.000000") "TraceTypeQuery1" false 0 "ForOneFrame"))
      (switch int _array_index
        (:0
          (Variables|Default|SetHeightUP (.Z (Math|Vector|BreakVector (.location _outhit_2)))))
        (:1
          (Variables|Default|SetHeightDown (.Z (Math|Vector|BreakVector (.location _outhit_2)))))
        (:2
          (Variables|Default|SetHeightRight (.Z (Math|Vector|BreakVector (.location _outhit_2)))))
        (:3
          (Variables|Default|SetHeightLeft (.Z (Math|Vector|BreakVector (.location _outhit_2)))))))
    (Variables|Default|SetNewVar_0 (Math|Vector|Normalize (Math|Vector|MakeVector (- (Variables|Default|GetHeightDown) (Variables|Default|GetHeightUP)) (- (Variables|Default|GetHeightLeft) (Variables|Default|GetHeightRight)) 0.0)))
    (bind _output_get (Variables|Default|SetNormal (Math|Vector|Normalize (Math|Vector|MakeVector (- (Variables|Default|GetHeightUP) (Variables|Default|GetHeightDown)) (- (Variables|Default|GetHeightRight) (Variables|Default|GetHeightLeft)) 2.0))))
    (Development|PrintString (Utilities|String|ToString(Vector) _output_get) true true "(R=1.000000,G=0.000000,B=0.153831,A=1.000000)")
    (Development|PrintString (Utilities|String|ToString(Vector) (Variables|Default|GetNewVar_0)) true true "(R=0.000000,G=0.319231,B=1.000000,A=1.000000)")
    (Rendering|Debug|DrawDebugLine (- (Variables|Default|GetCenter) "0, 0,500.000000") (+ (- (Variables|Default|GetCenter) "0, 0,500.000000") (* (Variables|Default|GetNormal) 5e+02)) "(R=0.000000,G=1.000000,B=0.040460,A=1.000000)" 15.0 9.0)
    (Rendering|Debug|DrawDebugLine (- (Variables|Default|GetCenter) "0, 0,500.000000") (+ (- (Variables|Default|GetCenter) "0, 0,500.000000") (* (Variables|Default|GetHitNormal) 2.5e+02)) "(R=1.000000,G=0.000000,B=0.172772,A=1.000000)" 15.0 9.0)
    (Rendering|Debug|DrawDebugLine (- (Variables|Default|GetCenter) "0, 0,500.000000") (+ (- (Variables|Default|GetCenter) "0, 0,500.000000") (* (Variables|Default|GetNewVar_0) 4e+02)) "(R=0.000000,G=0.185775,B=1.000000,A=1.000000)" 15.0 9.0)))

(fn ConstructionScript)