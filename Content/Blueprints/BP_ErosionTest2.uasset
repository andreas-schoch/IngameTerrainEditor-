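; BP_ErosionTest2 is a test actor, apparently for erosion, that triggers sculpting through its Sculpt member and lives for a limited time.
; Shortly after BeginPlay it calls SculptStart on Sculpt, then sets a lifespan so it destroys itself.
; Tick locks the Camera to a fixed world rotation, and a debug line drawn along the camera's backward axis is left disconnected.
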(event EventTick
  (params (DeltaSeconds :type Float%20%28single-precision%29))
  (Transformation|SetWorldRotation (Variables|Default|GetCamera) "-90.000000, 0, 0" false false))

(event EventBeginPlay
  (Utilities|FlowControl|Delay 0.2)
  (Class|SculptComponent|SculptStart (Variables|Default|GetSculpt))
  (Actor|SetLifeSpan 25.0))

(fn ConstructionScript)